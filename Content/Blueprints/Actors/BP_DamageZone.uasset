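; BP_DamageZone is a box-shaped volume that deals repeated damage to an actor inside it.
; Begin overlap stores the actor and starts a looping timer that sends DealDamageMessage with DamageAmount every DamageDealRate seconds.
; Only the latest entering actor is tracked, and any end overlap clears both that reference and the current timer handle.
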(event `OnDamageDeal`
  (bind _overlappingactor (`self.OverlappingActor`)
    (:`then`
      (message `/Game/Blueprints/Actors/BPI_DamageInteractions.DealDamage` _overlappingactor (`self.DamageAmount`)))
    (:`else`)))

(event `self.Box.OnComponentBeginOverlap`
  (params (OverlappedComponent :type "PrimitiveComponent Object Reference") (OtherActor :type "Actor Object Reference") (OtherComp :type "PrimitiveComponent Object Reference") (OtherBodyIndex :type Integer) (bFromSweep :type Boolean) (SweepResult :type "HitResult Structure (by ref)"))
  (set `self.OverlappingActor` OtherActor)
  (bind _returnvalue (`KismetSystemLibrary.K2_SetTimerDelegate` (delegate `OnDamageDeal`) (`self.DamageDealRate`) true))
  (set `self.DamageTimer` _returnvalue))

(event `self.Box.OnComponentEndOverlap`
  (params (OverlappedComponent :type "PrimitiveComponent Object Reference") (OtherActor :type "Actor Object Reference") (OtherComp :type "PrimitiveComponent Object Reference") (OtherBodyIndex :type Integer))
  (set `self.OverlappingActor` null)
  (`KismetSystemLibrary.K2_ClearAndInvalidateTimerHandle` (`self.DamageTimer`)))

(fn `UserConstructionScript`)