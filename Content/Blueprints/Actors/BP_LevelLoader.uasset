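; BP_LevelLoader is an actor that swaps streamed levels by index from its StreamLevels list.
; OnLoadNewLevel starts a non-blocking load of the chosen level and unloads the previous one from a parallel sequence branch.
; Once the latent load finishes, it records the new index and broadcasts completion with the level name and spawn point, converted to world space by offsetting from the loader's transform.
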(event `OnLoadNewLevel`
  (params (OnIndex :type Integer))
  (bind (_levelname _levelspawnpoint) (break `/Game/Base/Data/ST_LevelLoadData` (`|GetArrayItem` (`self.StreamLevels`) (`self.LoadedStreamLevelIndex`))))
  (set `self.LoadedStreamLevelIndex` OnIndex)
  (`|ExecutionSequence`
    (:`then_0`
      (`GameplayStatics.LoadStreamLevel` (`.LevelName_6_6F8417994132F8A403954FB778247C27` (break `/Game/Base/Data/ST_LevelLoadData` (`|GetArrayItem` (`self.StreamLevels`) (`self.LoadedStreamLevelIndex`)))) true)
      (set `self.PreviousStreamLevel` (`self.LoadedStreamLevelIndex`))
      (bind _outworldtransform (`self.ConvertRelativeToWorldTransform` _levelspawnpoint))
      (`self.OnLevelLoadComplete` (make `/Game/Base/Data/ST_LevelLoadData` _levelname _outworldtransform)))
    (:`then_1`
      (if (>= (`self.PreviousStreamLevel`) 0)
        (`GameplayStatics.UnloadStreamLevel` (`.LevelName_6_6F8417994132F8A403954FB778247C27` (break `/Game/Base/Data/ST_LevelLoadData` (`|GetArrayItem` (`self.StreamLevels`) (`self.PreviousStreamLevel`)))))))))

(fn `ConvertRelativeToWorldTransform`
  (params (InRelativeTransform :type "Transform Structure"))
  (returns (OutWorldTransform :type "Transform Structure"))
  (bind (_returnvalue_location _returnvalue_rotation) (`KismetMathLibrary.BreakTransform` (`self.GetTransform`)))
  (return (`KismetMathLibrary.MakeTransform` (+ (.location (`local.InRelativeTransform`)) _returnvalue_location) (`KismetMathLibrary.ComposeRotators` (.rotation (`local.InRelativeTransform`)) _returnvalue_rotation))))

(fn `UserConstructionScript`
  (locals (L_CurrentArrow :type "ArrowComponent Object Reference")))