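; BP_PlayerController is a player controller that possesses the player pawn when the game mode signals it.
; On BeginPlay it caches BP_GameMode and binds to that game mode's OnStartPlayerPosessing event.
; When the event delivers a valid pawn, the controller possesses it and then unbinds, so possession is a one-shot handoff driven by the game mode.
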(event `self.ReceiveBeginPlay`
  (`self.SetStartParams`))

(event `OnStartPlayerPosessing`
  (params (OfPlayerPawn :type "Pawn Object Reference"))
  (`self.PlayerPosessHandler` OfPlayerPawn))

(fn `PlayerPosessHandler`
  (params (InPlayerPawn :type "Pawn Object Reference"))
  (`local.InPlayerPawn`
    (:`then`
      (`|ExecutionSequence`
        (:`then_0`
          (`self.Possess` (`local.InPlayerPawn`)))
        (:`then_1`
          (bind _gamemode (`self.GameMode`)
            (:`then`
              (remove `/Game/Blueprints/BP_GameMode.OnStartPlayerPosessing` _gamemode (`|CreateDelegate` :!event `OnStartPlayerPosessing`)))
            (:`else`)))))
    (:`else`)))

(fn `SetStartParams`
  (`|ExecutionSequence`
    (:`then_0`
      (bind _asbp_game_mode (cast `/Game/Blueprints/BP_GameMode` (`GameplayStatics.GetGameMode`)))
      (set `self.GameMode` _asbp_game_mode))
    (:`then_1`
      (bind _gamemode (`self.GameMode`)
        (:`then`
          (add `/Game/Blueprints/BP_GameMode.OnStartPlayerPosessing` _gamemode (`|CreateDelegate` :!event `OnStartPlayerPosessing`)))
        (:`else`)))))

(fn `UserConstructionScript`)