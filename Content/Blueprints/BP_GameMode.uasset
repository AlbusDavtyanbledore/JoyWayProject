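; Game mode that sets up the main UI, player possession and level loading at game start.
; On BeginPlay it finds the tagged level loader, creates the main widget, broadcasts possession for the existing pawn and loads the first level.
; Event dispatchers relay UI level requests to the loader and announce load completion.
; It also toggles UI/game input mode and cursor; the code that spawns BP_Player is disconnected.
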(event `self.ReceiveBeginPlay`
  (`self.SetStartParams`))

(event `OnLevelLoad`
  (params (OnIndex :type Integer))
  (`self.LevelLoadHandler` OnIndex))

(event `OnLevelLoaded`
  (params (LevelLoadData :type "/Game/Base/Data/ST_LevelLoadData Structure"))
  (`self.OnLevelLoadCompleted` LevelLoadData))

(fn `Binds`
  (`|ExecutionSequence`
    (:`then_0`
      (bind _mainwidget (`self.MainWidget`)
        (:`then`
          (add `/Game/UI/BP_UI_Main.OnLevelPendingToLoad` _mainwidget (`|CreateDelegate` :!event `OnLevelLoad`)))
        (:`else`)))
    (:`then_1`
      (bind _levelloaderactor (`self.LevelLoaderActor`)
        (:`then`
          (add `/Game/Blueprints/Actors/BP_LevelLoader.OnLevelLoadComplete` _levelloaderactor (`|CreateDelegate` :!event `OnLevelLoaded`)))
        (:`else`)))))

(fn `GetLevelLoaderActor`
  (returns (Success :type Boolean) (LevelLoaderActor :type "/Game/Blueprints/Actors/BP_LevelLoader Object Reference"))
  (if (`KismetSystemLibrary.IsValid` (`self.LevelLoaderActor`))
    (return true (`self.LevelLoaderActor`))
    (else
      (return false null))))

(fn `LevelLoadHandler`
  (params (InIndex :type Integer))
  (`self.LevelLoaderActor`
    (:`then`
      (`/Game/Blueprints/Actors/BP_LevelLoader.OnLoadNewLevel` (`self.LevelLoaderActor`) (`local.InIndex`)))
    (:`else`)))

(fn `SetInputModeUI/Game`
  (params (State :type Boolean))
  (bind _output_get (set `self.bIsInUI` State))
  (if _output_get
    (`WidgetBlueprintLibrary.SetInputMode_GameAndUIEx` (`GameplayStatics.GetPlayerController` 0) (`self.MainWidget`))
    (set `PlayerController.bShowMouseCursor` true (`GameplayStatics.GetPlayerController` 0))
    (`self.OnUIActivation` true)
    (else
      (`WidgetBlueprintLibrary.SetInputMode_GameOnly` (`GameplayStatics.GetPlayerController` 0))
      (set `PlayerController.bShowMouseCursor` false (`GameplayStatics.GetPlayerController` 0))
      (`self.OnUIActivation` false))))

(fn `SetStartParams`
  (`|ExecutionSequence`
    (:`then_0`
      (bind _outactors (`GameplayStatics.GetAllActorsWithTag` "level_loader"))
      (bind _asbp_level_loader (cast `/Game/Blueprints/Actors/BP_LevelLoader` (`|GetArrayItem` _outactors)))
      (set `self.LevelLoaderActor` _asbp_level_loader))
    (:`then_1`
      (bind _returnvalue (`|CreateWidget` "/Game/UI/BP_UI_Main.BP_UI_Main_C" (`GameplayStatics.GetPlayerController` 0)))
      (bind _output_get (set `self.MainWidget` _returnvalue))
      (`UserWidget.AddToViewport` _output_get 0)
      (`WidgetBlueprintLibrary.SetInputMode_GameOnly` (`GameplayStatics.GetPlayerController` 0)))
    (:`then_2`
      (bind _asbp_player_controller (cast `/Game/Blueprints/BP_PlayerController` (`GameplayStatics.GetPlayerController` 0)))
      (set `self.PlayerController` _asbp_player_controller))
    (:`then_3`
      (`self.Binds`)
      (`self.SpawnPlayer`)
      (`self.LevelLoadHandler` 0))))

(fn `SpawnPlayer`
  (`self.LevelLoaderActor`
    (:`then`
      (`self.PlayerController`
        (:`then`
          (`|ExecutionSequence`
            (:`then_0`
              (add `self.OnStartPlayerPosessing` (`|CreateDelegate` (`self.PlayerController`) :!event `OnStartPlayerPosessing`)))
            (:`then_1`
              (`self.OnStartPlayerPosessing` (`GameplayStatics.GetPlayerPawn` 0)))))
        (:`else`)))
    (:`else`)))

(fn `UserConstructionScript`)